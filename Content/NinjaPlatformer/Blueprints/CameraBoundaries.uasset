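; CameraBoundaries is a placeable actor that defines a rectangular camera boundary area in the X-Z plane with a Box component.
; The construction script sizes the box to half of Corner and offsets it by its extent, anchoring its lower corner at the actor origin.
; GetBoundaries computes from zero constants rather than Corner, so BottomLeft and TopRight both equal the actor location.
; BeginPlay prints Corner.
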(event EventBeginPlay
  (Development|PrintString (Utilities|String|ToString(Vector) (Variables|Default|GetCorner))))

(fn ConstructionScript
  (bind _box (Variables|Default|GetBox))
  (bind _corner (Variables|Default|GetCorner))
  (bind _returnvalue (/ _corner 2.0))
  (bind _boxextent (Variables|/Script/Engine.BoxComponent|GetBoxExtent _box))
  (Utilities|FlowControl|Sequence
    (:then_0
      (Components|Box|SetBoxExtent (Variables|Default|GetBox) (Math|Vector|MakeVector (.x _returnvalue) 1e+02 (.z _returnvalue)) true))
    (:then_1
      (Transformation|SetRelativeLocation _box (Math|Vector|MakeVector (.x _boxextent) 0.0 (.z _boxextent)) false false))))

(fn GetBoundaries
  (bind _returnvalue (Transformation|GetActorLocation))
  (bind _returnvalue_2 (/ "" 2.0))
  (bind _returnvalue_3 (Math|Vector|MakeVector (.x _returnvalue_2) 0.0 (.y _returnvalue_2)))
  (return (- _returnvalue _returnvalue_3) (+ _returnvalue _returnvalue_3)))