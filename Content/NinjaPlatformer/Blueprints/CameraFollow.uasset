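; Side-scrolling follow camera actor that makes itself the first player's view target and tracks that player's pawn.
; The construction script pins it to a configurable Y depth with a fixed rotation.
; A looping timer acquires the player pawn whenever the stored reference is invalid.
; Each tick interpolates X and Z toward the pawn at a high speed, keeping Y unchanged.
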(event Custom|CheckCharacter
  (bind _returnvalue (Game|Player|GetPlayerPawn 0))
  (Utilities|IsValid (Variables|Default|GetFollowPawn)
    (:Is%20Not%20Valid
      (Utilities|IsValid _returnvalue
        (:Is%20Valid
          (Variables|Default|SetFollowPawn _returnvalue))))))

(event Custom|UpdateLocation
  (params (DeltaTime :type Float%20%28single-precision%29))
  (bind _returnvalue (Transformation|GetActorLocation))
  (bind _followpawn (Variables|Default|GetFollowPawn))
  (bind _returnvalue_2 (Transformation|GetActorLocation _followpawn))
  (Utilities|IsValid _followpawn
    (:Is%20Valid
      (Transformation|SetActorLocation (Math|Interpolation|VInterpTo (Math|Vector|MakeVector (.x _returnvalue) (.y _returnvalue) (.z _returnvalue)) (Math|Vector|MakeVector (.x _returnvalue_2) (.y _returnvalue) (.z _returnvalue_2)) DeltaTime 1e+02) false false))))

(event EventBeginPlay
  (Utilities|Time|SetTimerbyFunctionName 0 "CheckCharacter" 0.2 true)
  (Game|Player|SetViewTargetwithBlend (Game|GetPlayerController 0) self 0.0 "VTBlend_Linear" 0.0 false))

(event EventTick
  (params (DeltaSeconds :type Float%20%28single-precision%29))
  (CallFunction|UpdateLocation DeltaSeconds))

(fn ConstructionScript
  (bind _returnvalue (Transformation|GetActorLocation))
  (Transformation|SetActorLocation (Math|Vector|MakeVector (.x _returnvalue) (Variables|Default|GetYLocation) (.z _returnvalue)) false false)
  (Transformation|SetActorRotation "0,270.000000, 0"))